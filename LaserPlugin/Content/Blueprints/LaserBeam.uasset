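; Laser beam actor that stretches to the first object it hits and notifies mirrors so they can update reflections.
; Tick sphere-traces forward, ignoring laser sources, other beams and any owning mirror, and only acts when impact point or normal changes.
; Mirrors get impact data through AC_Reflect and BI_MirrorUpdate, plus an end-overlap update when the beam leaves them.
; The construction script runs a similar trace to size the beam and end cap.
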(event Custom|ImplementOwnMirror
  (params (Mirror :type Actor%20Object%20Reference))
  (bind _exempt (Variables|Default|GetExempt))
  ;[0.15 0.15 0.15 0.5] All this is just setting what actors to exclude from the sphere trace, if you want the laser to ignore something, you gotta add it to "exempt" array
  (Utilities|Array|Clear _exempt)
  (bind _outactors (Actor|GetAllActorsOfClass "/LaserPlugin/Blueprints/LaserSource.LaserSource_C"))
  (Utilities|Array|AppendArray _exempt _outactors)
  (bind _outactors_2 (Actor|GetAllActorsOfClass "LaserBeam_C"))
  (Utilities|Array|AppendArray _exempt _outactors_2)
  (Utilities|Array|Add _exempt Mirror)
  (Variables|Default|SetPrevImpact "1111111.000000,0.000000,0.000000"))

(event EventTick
  (params (DeltaSeconds :type Float%20%28single-precision%29))
  (bind _self self)
  (bind _previousactor (Variables|Default|GetPreviousActor))
  (bind _previousactor_2 (Variables|Default|GetPreviousActor))
  (bind _returnvalue (Actor|GetComponentbyClass _previousactor "/LaserPlugin/Blueprints/AC_Reflect.AC_Reflect_C"))
  (bind (_hitactor _location _impactnormal _distance _returnvalue_2) (|SphereTrace))
  (|ComparingPastLocation _location _impactnormal
    (:else
      ;[0.15 0.15 0.15 0.5] Update prev hit details, then check if hitting a new object entirely
      (Variables|Default|SetPrevImpact _location)
      (Variables|Default|SetPrevNormal _impactnormal)
      (if (not (== _hitactor _previousactor_2))
        (|CallingReflectUpdate _previousactor_2 _hitactor _previousactor_2))
      (if _returnvalue_2
        (Variables|Default|SetDistanceToScale (+ _distance -1.0))
        ;[0.15 0.15 0.15 0.5] If hitting a mirror -> true
        (if (Utilities|DoesObjectImplementInterface (Actor|GetComponentbyClass _hitactor "/LaserPlugin/Blueprints/AC_Reflect.AC_Reflect_C") "/LaserPlugin/Blueprints/BI_MirrorUpdate.BI_MirrorUpdate_C")
          ;[0.08333 0.08333 0.08333 0.5] This also calls the reflect update
          (Default|CallUpdate (Actor|GetComponentbyClass _hitactor "/LaserPlugin/Blueprints/AC_Reflect.AC_Reflect_C") _self _location _impactnormal false)
          (else
            (if (Utilities|IsValid (Variables|Default|GetPreviousActor)) :!label _label
              (if (Utilities|DoesObjectImplementInterface _returnvalue "/LaserPlugin/Blueprints/BI_MirrorUpdate.BI_MirrorUpdate_C")
                (Default|CallUpdate _returnvalue _self _location _impactnormal true)))))
        (else
          (Variables|Default|SetDistanceToScale (+ (Variables|Default|GetLaserMaxLength) -1.0))
          (goto _label)))
      (|SettingLaserLength))))

(event EventBeginPlay
  (bind _exempt (Variables|Default|GetExempt))
  ;[0.15 0.15 0.15 0.5] All this is just setting what actors to exclude from the sphere trace, if you want the laser to ignore something, you gotta add it to "exempt" array
  (bind _outactors (Actor|GetAllActorsOfClass "/LaserPlugin/Blueprints/LaserSource.LaserSource_C"))
  (Utilities|Array|AppendArray _exempt _outactors)
  (bind _outactors_2 (Actor|GetAllActorsOfClass "LaserBeam_C"))
  (Utilities|Array|AppendArray _exempt _outactors_2)
  (Variables|Default|SetPrevImpact "1111111.000000,0.000000,0.000000"))

(fn ConstructionScript
  (bind _returnvalue (Transformation|GetActorLocation))
  (bind _beam (Variables|Default|GetBeam))
  (bind _laserwidth (Variables|Default|GetLaserWidth))
  (bind _relativescale3d (Variables|/Script/Engine.SceneComponent|GetRelativeScale3D _beam))
  (Transformation|SetRelativeScale3D (Variables|Default|GetBeam) (Math|Vector|MakeVector _laserwidth _laserwidth 0.0))
  (Transformation|SetRelativeScale3D (Variables|Default|GetLaserEnd) (Math|Vector|MakeVector _laserwidth _laserwidth _laserwidth))
  (bind (_outhit _returnvalue_2) (Collision|SphereTraceByChannel _returnvalue (+ _returnvalue (* (Transformation|GetActorForwardVector) (Variables|Default|GetLaserMaxLength))) (* 5e+01 (Variables|Default|GetLaserWidth)) "TraceTypeQuery1" false 0 "None"))
  (if _returnvalue_2
    (Variables|Default|SetDistanceToScale (+ (.Distance (Collision|BreakHitResult _outhit)) 2.0))
    (else
      (Variables|Default|SetDistanceToScale (+ (Variables|Default|GetLaserMaxLength) 2.0))))
  (Transformation|SetRelativeScale3D _beam (Math|Vector|MakeVector (.x _relativescale3d) (.y _relativescale3d) (/ (Variables|Default|GetDistanceToScale) 1e+02)))
  (Transformation|SetRelativeLocation (Variables|Default|GetBeam) (Math|Vector|MakeVector (/ (Variables|Default|GetDistanceToScale) 2.0) 0.0 0.0) false true)
  (Transformation|SetRelativeLocation (Variables|Default|GetLaserEnd) (Math|Vector|MakeVector (.x (Math|Conversions|ToVector(Float) (Variables|Default|GetDistanceToScale))) 0.0 0.0) false true))