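; Laser relay actor that switches a list of linked actors on and off when a LaserBeam enters or leaves its box collision.
; Begin and end overlap swap the sphere's material between active and inactive looks as a status light.
; Each actor in AllActorsToActivate receives the activate or deactivate message through BI_RelayInterface, with a printed warning for any actor lacking the interface.
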(event OnComponentBeginOverlap(BoxCollision)
  (params (OverlappedComponent :type Primitive%20Component%20Object%20Reference) (OtherActor :type Actor%20Object%20Reference) (OtherComp :type Primitive%20Component%20Object%20Reference) (OtherBodyIndex :type Integer) (bFromSweep :type Boolean) (SweepResult :type Hit%20Result%20Structure%20%28by%20ref%29))
  ;[0.15 0.15 0.15 0.5] OneActivated
  (if (Class|GameplayStatics|ObjectIsA OtherActor "/LaserPlugin/Blueprints/LaserBeam.LaserBeam_C")
    ;[0.15 0.15 0.15 0.5] Cosmetic, sets light to green
    (Rendering|Material|SetMaterial (Variables|Default|GetSphere) 0 "/LaserPlugin/Customize/M_RelayActive.M_RelayActive")
    ;[0.15 0.15 0.15 0.5] Check each actor in the list actually has a function to be activated
    (for _array_element (Variables|Default|GetAllActorsToActivate)
      (if (Utilities|DoesObjectImplementInterface _array_element "/LaserPlugin/Blueprints/BI_RelayInterface.BI_RelayInterface_C")
        ;[0.15 0.15 0.15 0.5] Sends message to activate the actors function
        (Class|BIRelayInterface|RelayActivated(Message) _array_element)
        (else
          (Development|PrintString "An actor you are trying to activate does not have the \"BI Relay Interface\" added."))))))

(event OnComponentEndOverlap(BoxCollision)
  (params (OverlappedComponent :type Primitive%20Component%20Object%20Reference) (OtherActor :type Actor%20Object%20Reference) (OtherComp :type Primitive%20Component%20Object%20Reference) (OtherBodyIndex :type Integer))
  ;[0.15 0.15 0.15 0.5] OnDeActivated
  (if (Class|GameplayStatics|ObjectIsA OtherActor "/LaserPlugin/Blueprints/LaserBeam.LaserBeam_C")
    (Rendering|Material|SetMaterial (Variables|Default|GetSphere) 0 "/LaserPlugin/Customize/M_RelayUnactive.M_RelayUnactive")
    (for _array_element (Variables|Default|GetAllActorsToActivate)
      (if (Utilities|DoesObjectImplementInterface _array_element "/LaserPlugin/Blueprints/BI_RelayInterface.BI_RelayInterface_C")
        (Class|BIRelayInterface|RelayDeactivated(Message) _array_element)
        (else
          (Development|PrintString "An actor you are trying to deactivate does not have the \"BI Relay Interface\" added."))))))

(fn ConstructionScript)