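; Actor component that reflects laser beams off its owner, spawning a mirrored LaserBeam at the impact point.
; Each update destroys the calling laser's previous reflection, then respawns one unless the overlap ended or ShouldDeflect fails, tracking beams in a map keyed by source actor.
; An Update flag with a zero-length Delay limits processing to one call per tick.
; ShouldDeflect's facing and ReflectAllSides check is left unconnected.
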(event Custom|UpdateReflections
  (params (CallingActor :type Actor%20Object%20Reference) (ImpactPoint :type Vector) (ImpactNormal :type Vector) (DidEndOverlap? :type Boolean))
  (if (Variables|Default|GetUpdate?)
    (Variables|Default|SetUpdate? false)
    (if DidEndOverlap?
      (CallFunction|DestroyReflected CallingActor :!label _label)
      (else
        (if (.ReturnValue (Utilities|Map|Find (Variables|Default|GetLaserBeams) CallingActor))
          (CallFunction|DestroyReflected CallingActor))
        (if (Utilities|ShouldDeflect? CallingActor ImpactNormal)
          (CallFunction|CreateLaser CallingActor ImpactPoint ImpactNormal)
          (else
            (goto _label)))))
    (Utilities|FlowControl|Delay 0.0)
    (Variables|Default|SetUpdate? true)))

(event Custom|DestroyReflected
  (params (DestroyedActor :type Actor%20Object%20Reference))
  (bind _laserbeams (Variables|Default|GetLaserBeams))
  (bind (_value _returnvalue) (Utilities|Map|Find _laserbeams DestroyedActor))
  (if _returnvalue
    (Actor|DestroyActor _value)
    (Utilities|Map|Remove _laserbeams DestroyedActor)))

(event Custom|Create%20Laser
  (params (Key :type Actor%20Object%20Reference) (ImpactPoint :type Vector) (ImpactNormal :type Vector))
  (Game|BindEventtoOnDestroyed Key (EventDispatchers|CreateEvent :!event Custom|DestroyReflected))
  (bind _returnvalue (Game|SpawnActorfromClass "/LaserPlugin/Blueprints/LaserBeam.LaserBeam_C" (Math|Transform|MakeTransform ImpactPoint (Math|Conversions|RotationFromXVector (Math|Vector|MirrorVectorbyNormal (Math|Vector|Normalize (Transformation|GetActorForwardVector Key)) ImpactNormal)) "1.000000,1.000000,1.000000") "Undefined" "MultiplyWithRoot" 0 0))
  (Utilities|Map|Add (Variables|Default|GetLaserBeams) Key _returnvalue)
  (Default|ImplementOwnMirror _returnvalue (Components|GetOwner)))

(event EventCallUpdate
  (params (CallingActor :type Actor%20Object%20Reference) (ImpactPoint :type Vector :default "0, 0, 0") (ImpactNormal :type Vector :default "0, 0, 0") (DidEndOverlap? :type Boolean))
  (CallFunction|UpdateReflections CallingActor ImpactPoint ImpactNormal DidEndOverlap?))