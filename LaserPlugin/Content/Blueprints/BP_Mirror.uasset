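; BP_Mirror is an interactable mirror that the player can rotate or carry, driven by its InteractionComponent.
; A long interaction nudges the actor's yaw by a small step.
; When CanGrab is true, a short interaction casts the instigator to BP_GAD2010 and toggles carrying through that character's CurrentlyGrabbing flag.
; Carrying attaches it to the character's mesh, disables cube collision and slows walking; dropping detaches it and restores both.
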(event OnLongInteraction(InteractionComponent)
  (params (Instigator :type Actor%20Object%20Reference) (Phase :type InteractionPhase%20Enum :default "NewEnumerator0") (Delta :type Float%20%28double-precision%29))
  (bind _returnvalue (Transformation|GetActorRotation))
  ;[0.15 0.15 0.15 0.5] On hold, rotate the object
  (Transformation|SetActorRotation (Math|Rotator|MakeRotator (.roll _returnvalue) (.pitch _returnvalue) (+ (.yaw _returnvalue) 0.5))))

(event OnShortInteraction(InteractionComponent)
  (params (Instigator :type Actor%20Object%20Reference))
  (bind _cube (Variables|Default|GetCube))
  ;[0.15 0.15 0.15 0.5] On press, pick up the object
  (if (Variables|Default|GetCanGrab?)
    ;[0.15 0.15 0.15 0.5] If this returns an error, you are using a different character. Just replace the cast with a cast to your character
    (bind _asbp_gad2010 (Utilities|Casting|CastToBP_GAD2010 Instigator))
    (if (Variables|/Game/Base/Character/Blueprints/BP_GAD2010.BP_GAD2010_C|GetCurrentlyGrabbing? _asbp_gad2010)
      (Variables|/Game/Base/Character/Blueprints/BP_GAD2010.BP_GAD2010_C|SetCurrentlyGrabbing? _asbp_gad2010 false)
      (Variables|/Script/Engine.CharacterMovementComponent|SetMaxWalkSpeed (Variables|/Script/Engine.Character|GetCharacterMovement _asbp_gad2010) (/ (Variables|/Script/Engine.CharacterMovementComponent|GetMaxWalkSpeed (Variables|/Script/Engine.Character|GetCharacterMovement _asbp_gad2010)) 0.7))
      (Transformation|DetachFromActor "KeepWorld" "KeepWorld" "KeepWorld")
      (Collision|SetCollisionEnabled _cube "QueryAndPhysics")
      (Transformation|SetRelativeLocation (Variables|Default|GetCube) "40.000000,0.000000,100.000000" false false)
      (else
        (Variables|/Game/Base/Character/Blueprints/BP_GAD2010.BP_GAD2010_C|SetCurrentlyGrabbing? _asbp_gad2010 true)
        (Variables|/Script/Engine.CharacterMovementComponent|SetMaxWalkSpeed (Variables|/Script/Engine.Character|GetCharacterMovement _asbp_gad2010) (* (Variables|/Script/Engine.CharacterMovementComponent|GetMaxWalkSpeed (Variables|/Script/Engine.Character|GetCharacterMovement _asbp_gad2010)) 0.7))
        (Transformation|AttachComponentToComponent (Variables|/Script/Engine.Character|GetMesh _asbp_gad2010) "None" "SnapToTarget" "SnapToTarget" "KeepRelative" true)
        (Collision|SetCollisionEnabled _cube "NoCollision")
        (Transformation|SetRelativeLocation (Variables|Default|GetCube) "40.000000,0.000000,100.000000" false true)
        (Transformation|SetActorRelativeRotation "0.000000,90.000000,0.000000")))))

(fn ConstructionScript)